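; Detonator Blueprint for an interactable detonator that fires only once its required components have been placed.
; On BeginPlay and on each Interact, it checks the GameInstance flags for antenna, TNT and receiver, latching CanDetonate when all are set.
; Interact then either activates the root component of the referenced PEffect and prints a boom message, or prints that it is not ready.
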(event EventBeginPlay
  (bind _returnvalue (Game|GetGameInstance))
  (if (not (Variables|Default|GetcanDetonate))
    (bind _asgame_instace (Utilities|Casting|CastToGameInstace _returnvalue))
    (if (Variables|/Game/InventorySystem/GameInstace.GameInstace_C|GetisAntellaPlaced _asgame_instace)
      (bind _asgame_instace_2 (Utilities|Casting|CastToGameInstace _returnvalue))
      (if (Variables|/Game/InventorySystem/GameInstace.GameInstace_C|GetisTNTPlaced _asgame_instace_2)
        (bind _asgame_instace_3 (Utilities|Casting|CastToGameInstace _returnvalue))
        (if (Variables|/Game/InventorySystem/GameInstace.GameInstace_C|GetisRecieverPlaced _asgame_instace_3)
          (Variables|Default|SetcanDetonate true)
          (Development|PrintString "Ready to Detonate"))))))

(event Collision|EventActorBeginOverlap
  (params (OtherActor :type Actor%20Object%20Reference)))

(event EventTick
  (params (DeltaSeconds :type Float%20%28single-precision%29)))

(event EventInteract
  (bind _returnvalue (Game|GetGameInstance))
  (Utilities|FlowControl|Sequence
    (:then_0
      (if (not (Variables|Default|GetcanDetonate))
        (bind _asgame_instace (Utilities|Casting|CastToGameInstace _returnvalue))
        (if (Variables|/Game/InventorySystem/GameInstace.GameInstace_C|GetisAntellaPlaced _asgame_instace)
          (bind _asgame_instace_2 (Utilities|Casting|CastToGameInstace _returnvalue))
          (if (Variables|/Game/InventorySystem/GameInstace.GameInstace_C|GetisTNTPlaced _asgame_instace_2)
            (bind _asgame_instace_3 (Utilities|Casting|CastToGameInstace _returnvalue))
            (if (Variables|/Game/InventorySystem/GameInstace.GameInstace_C|GetisRecieverPlaced _asgame_instace_3)
              (Variables|Default|SetcanDetonate true)
              (Development|PrintString "Ready to Detonate"))))))
    (:then_1
      (if (Variables|Default|GetcanDetonate)
        (Development|PrintString "boom!")
        (Components|Activation|Activate (Variables|/Script/Engine.Actor|GetRootComponent (Variables|Default|GetpEffect)) false)
        (else
          (Development|PrintString "Not ready yet!"))))))

(fn ConstructionScript)