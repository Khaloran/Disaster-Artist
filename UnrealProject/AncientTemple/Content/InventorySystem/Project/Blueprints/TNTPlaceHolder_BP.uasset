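; Interactable TNT placeholder that the player fills in when carrying TNT.
; On Interact, it asks the player character's inventory manager whether at least one of the required item is held.
; If so, it swaps its mesh to the TNT material, flags TNT as placed in the GameInstance and unhides its Wires actors.
; Otherwise it only prints a reminder; the inventory check is not followed by any item removal.
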(event EventBeginPlay)

(event Collision|EventActorBeginOverlap
  (params (OtherActor :type Actor%20Object%20Reference)))

(event EventInteract
  (bind _asch_inventory_system_character (Utilities|Casting|CastToCH_InventorySystemCharacter (Game|GetPlayerCharacter 0)))
  (bind _inventorymanagercomponent (CallFunction|GetInventoryManager _asch_inventory_system_character))
  (bind _hadenough_ (Default|CheckItemAmmount _inventorymanagercomponent "NewEnumerator3" 1))
  (if _hadenough_
    (Development|PrintString "TNT in stock!")
    (Rendering|Material|SetMaterial (Variables|Debug|GetStaticMeshComponent) 0 (Variables|Default|GetTNTMaterial))
    (bind _asgame_instace (Utilities|Casting|CastToGameInstace (Game|GetGameInstance)))
    (Variables|/Game/InventorySystem/GameInstace.GameInstace_C|SetisTNTPlaced _asgame_instace true)
    (for _array_element (Variables|Default|Getwires)
      (Rendering|SetActorHiddenInGame _array_element false))
    (else
      (Development|PrintString "Go get the TNT dummy"))))

(fn ConstructionScript)