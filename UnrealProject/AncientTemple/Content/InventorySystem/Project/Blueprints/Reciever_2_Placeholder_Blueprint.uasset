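; Placeholder actor for a receiver slot that the player interacts with to place a receiver from their inventory.
; On Interact it asks the player character's inventory manager whether one of the required item is held.
; If so, it swaps the mesh material and sets the receiver-placed flag on the game instance; otherwise it prints a debug message telling the player to fetch one.
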(event EventBeginPlay)

(event Collision|EventActorBeginOverlap
  (params (OtherActor :type Actor%20Object%20Reference)))

(event EventTick
  (params (DeltaSeconds :type Float%20%28single-precision%29)))

(event EventInteract
  (bind _asch_inventory_system_character (Utilities|Casting|CastToCH_InventorySystemCharacter (Game|GetPlayerCharacter 0)))
  (bind _inventorymanagercomponent (CallFunction|GetInventoryManager _asch_inventory_system_character))
  (bind _hadenough_ (Default|CheckItemAmmount _inventorymanagercomponent "NewEnumerator1" 1))
  (if _hadenough_
    (Development|PrintString "Reciever in stock!")
    (Rendering|Material|SetMaterial (Variables|Debug|GetStaticMeshComponent) 0 (Variables|Default|GetNewVar_0))
    (bind _asgame_instace (Utilities|Casting|CastToGameInstace (Game|GetGameInstance)))
    (Variables|/Game/InventorySystem/GameInstace.GameInstace_C|SetisRecieverPlaced _asgame_instace true)
    (else
      (Development|PrintString "Go get the reciver dummy"))))

(fn ConstructionScript)